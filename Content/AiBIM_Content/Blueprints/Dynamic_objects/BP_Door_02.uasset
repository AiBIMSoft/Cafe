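; BP_Door_02 is an automatic double door that swings open when something overlaps its box collision and closes when the overlap ends.
; The DoorOpen timeline scales Angle1 and Angle2 to set each leaf's relative yaw, playing forward to open and reversing to close.
; A new audio component plays on opening and again after a short delay on closing, when Reverse is also called a second time.
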(event OnComponentBeginOverlap(BoxCollision)
  (params (OverlappedComponent :type Primitive%20Component%20Object%20Reference) (OtherActor :type Actor%20Object%20Reference) (OtherComp :type Primitive%20Component%20Object%20Reference) (OtherBodyIndex :type Integer) (bFromSweep :type Boolean) (SweepResult :type Hit%20Result%20Structure%20%28by%20ref%29))
  ;[1 1 1] Door Open/Close
  (bind _returnvalue (AddComponent|AddAudioComponent false))
  (Audio|Components|Audio|Play _returnvalue 0.0)
  (Audio|Components|Audio|AdjustVolume _returnvalue 0.0 1.0 "Linear" :!class /Script/Engine.AudioComponent)
  (bind _newtrack_0 (Timeline|Door%20open Play)
    (:Update
      (Transformation|SetRelativeRotation (Variables|Default|GetDoor1) (Math|Rotator|MakeRotator 0.0 0.0 (* _newtrack_0 (Variables|Default|GetAngle1))) false false)
      (Transformation|SetRelativeRotation (Variables|Default|GetDoor2) (Math|Rotator|MakeRotator 0.0 0.0 (* _newtrack_0 (Variables|Default|GetAngle2))) false false))))

(event OnComponentEndOverlap(BoxCollision)
  (params (OverlappedComponent :type Primitive%20Component%20Object%20Reference) (OtherActor :type Actor%20Object%20Reference) (OtherComp :type Primitive%20Component%20Object%20Reference) (OtherBodyIndex :type Integer))
  ;[1 1 1] Door Open/Close
  (Utilities|FlowControl|Sequence
    (:then_0
      (bind _newtrack_0 (Timeline|Door%20open Reverse)
        (:Update
          (Transformation|SetRelativeRotation (Variables|Default|GetDoor1) (Math|Rotator|MakeRotator 0.0 0.0 (* _newtrack_0 (Variables|Default|GetAngle1))) false false)
          (Transformation|SetRelativeRotation (Variables|Default|GetDoor2) (Math|Rotator|MakeRotator 0.0 0.0 (* _newtrack_0 (Variables|Default|GetAngle2))) false false))))
    (:then_1
      (Utilities|FlowControl|Delay 1.2)
      (bind _returnvalue (AddComponent|AddAudioComponent false))
      (Audio|Components|Audio|Play _returnvalue 0.0)
      (Audio|Components|Audio|AdjustVolume _returnvalue 0.0 1.0 "Linear" :!class /Script/Engine.AudioComponent)
      (Timeline|Door%20open Reverse))))

(fn ConstructionScript)