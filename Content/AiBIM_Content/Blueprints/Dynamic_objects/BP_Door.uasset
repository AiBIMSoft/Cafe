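; BP_Door is an automatic double door that opens when something enters its box collision and closes when it leaves.
; The DoorAnim timeline plays on overlap begin and reverses on overlap end, rotating two handles and the left and right panels by scaling its tracks with angle variables.
; The same 2D door sound plays immediately on opening and after a short delay on closing.
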(event OnComponentBeginOverlap(BoxCollision)
  (params (OverlappedComponent :type Primitive%20Component%20Object%20Reference) (OtherActor :type Actor%20Object%20Reference) (OtherComp :type Primitive%20Component%20Object%20Reference) (OtherBodyIndex :type Integer) (bFromSweep :type Boolean) (SweepResult :type Hit%20Result%20Structure%20%28by%20ref%29))
  ;[1 1 1] Door Open/Close
  (Audio|PlaySound2D "/Game/BPARCHVIZ_COURSEFILES/THIRD_PART/AUDIOS/S_Closedoor1_Cue.S_Closedoor1_Cue" 1.0 1.0 0.0 0 0)
  (bind (_direction _dooropen_close _handle) (Timeline|DoorAnim Play)
    (:Update
      (Transformation|SetRelativeRotation (Variables|Default|GetHandle2) (Math|Rotator|MakeRotator (* _handle (Variables|Default|GetDoorHandle1)) 0.0 0.0) false false)
      (Transformation|SetRelativeRotation (Variables|Default|GetHandle1) (Math|Rotator|MakeRotator 0.0 (* _handle (Variables|Default|GetDoorHandle1)) 0.0) false false)
      (Transformation|SetRelativeRotation (Variables|Default|GetDoor_L) (Math|Rotator|MakeRotator 0.0 0.0 (* _dooropen_close (Variables|Default|GetDoorAngle1))) false false)
      (Transformation|SetRelativeRotation (Variables|Default|GetDoor_R) (Math|Rotator|MakeRotator 0.0 0.0 (* _dooropen_close (Variables|Default|GetDoorAngle2))) false false))))

(event OnComponentEndOverlap(BoxCollision)
  (params (OverlappedComponent :type Primitive%20Component%20Object%20Reference) (OtherActor :type Actor%20Object%20Reference) (OtherComp :type Primitive%20Component%20Object%20Reference) (OtherBodyIndex :type Integer))
  ;[1 1 1] Door Open/Close
  (Utilities|FlowControl|Sequence
    (:then_0
      (bind (_direction _dooropen_close _handle) (Timeline|DoorAnim Reverse)
        (:Update
          (Transformation|SetRelativeRotation (Variables|Default|GetHandle2) (Math|Rotator|MakeRotator (* _handle (Variables|Default|GetDoorHandle1)) 0.0 0.0) false false)
          (Transformation|SetRelativeRotation (Variables|Default|GetHandle1) (Math|Rotator|MakeRotator 0.0 (* _handle (Variables|Default|GetDoorHandle1)) 0.0) false false)
          (Transformation|SetRelativeRotation (Variables|Default|GetDoor_L) (Math|Rotator|MakeRotator 0.0 0.0 (* _dooropen_close (Variables|Default|GetDoorAngle1))) false false)
          (Transformation|SetRelativeRotation (Variables|Default|GetDoor_R) (Math|Rotator|MakeRotator 0.0 0.0 (* _dooropen_close (Variables|Default|GetDoorAngle2))) false false))))
    (:then_1
      (Utilities|FlowControl|Delay 1.75)
      (Audio|PlaySound2D "/Game/BPARCHVIZ_COURSEFILES/THIRD_PART/AUDIOS/S_Closedoor1_Cue.S_Closedoor1_Cue" 1.0 1.0 0.0 0 0))))

(fn ConstructionScript)