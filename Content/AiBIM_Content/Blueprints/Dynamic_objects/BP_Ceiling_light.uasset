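; BP_Ceiling_light is an interactable ceiling light fixture that the player can switch on and off.
; Interact runs a FlipFlop that toggles twelve point lights between the Intensity variable and zero, swapping a mesh material between emissive and white plastic.
; Its prompt widget starts hidden, appears on WidgetInteraction, and hides again through the first-person character's IsNotHitting dispatcher, bound at BeginPlay.
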(event Custom|Hide%20Widget
  ;[1 1 1] Show/Hide Widget
  (Rendering|SetVisibility (Variables|Default|GetWBP_Light) false false))

(event EventWidgetInteraction
  ;[1 1 1] Show/Hide Widget
  (Rendering|SetVisibility (Variables|Default|GetWBP_Light) true false))

(event EventBeginPlay
  (Utilities|FlowControl|Sequence
    (:then_0
      ;[1 1 1] Set widget visibility
      (Rendering|SetVisibility (Variables|Default|GetWBP_Light) false false)
      ;[1 1 1] Get first person character Ref
      (bind _asbp_first_person_character (Utilities|Casting|CastToBP_FirstPersonCharacter (Game|GetPlayerCharacter 0)))
      (Variables|Default|SetBP_FirstPersonCharacter _asbp_first_person_character))
    (:then_1
      ;[1 1 1] Show/Hide Widget
      (EventDispatchers|BindEventtoIsNotHitting (Variables|Default|GetBP_FirstPersonCharacter) (delegate Custom|Hide%20Widget)))))

(event EventInteract
  (bind _staticmesh (Variables|Default|GetStaticMesh))
  ;[1 1 1] Light on/off
  (Utilities|FlowControl|FlipFlop
    (:A
      (Rendering|Components|Light|SetIntensity (Variables|Default|GetPointLight5) (Variables|Default|GetIntensity))
      (Rendering|Material|SetMaterial _staticmesh 2 "/Game/Material/Emissive_3.Emissive_3"))
    (:B
      (Rendering|Components|Light|SetIntensity (Variables|Default|GetPointLight7) 0.0)
      (Rendering|Material|SetMaterial _staticmesh 2 "/Game/Material/M_WhitePlastic_Inst.M_WhitePlastic_Inst"))))

(fn ConstructionScript)