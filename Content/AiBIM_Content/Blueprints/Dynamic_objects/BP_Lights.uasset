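; BP_Lights is an interactable light switch that toggles a group of room lights between bright and dimmed states.
; Interact plays a click and alternates two timelines that rotate the switch, then set rect and up/down light intensities and swap fixture materials.
; A widget shows on border overlap or WidgetInteraction and hides on overlap end or HideWidget; the character's HideWidget binding is never executed.
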(event OnComponentBeginOverlap(Collisionborder)
  (params (OverlappedComponent :type Primitive%20Component%20Object%20Reference) (OtherActor :type Actor%20Object%20Reference) (OtherComp :type Primitive%20Component%20Object%20Reference) (OtherBodyIndex :type Integer) (bFromSweep :type Boolean) (SweepResult :type Hit%20Result%20Structure%20%28by%20ref%29))
  ;[1 1 1] Widget Appear
  (Rendering|SetVisibility (Variables|Default|GetWBP_Light) true false))

(event OnComponentEndOverlap(Collisionborder)
  (params (OverlappedComponent :type Primitive%20Component%20Object%20Reference) (OtherActor :type Actor%20Object%20Reference) (OtherComp :type Primitive%20Component%20Object%20Reference) (OtherBodyIndex :type Integer))
  ;[1 1 1] Widget Appear
  (Rendering|SetVisibility (Variables|Default|GetWBP_Light) false false))

(event Custom|Hide%20Widget
  ;[1 1 1] Show/Hide Widget
  (Rendering|SetVisibility (Variables|Default|GetWBP_Light) false false))

(event EventWidgetInteraction
  ;[1 1 1] Show/Hide Widget
  (Rendering|SetVisibility (Variables|Default|GetWBP_Light) true false))

(event EventBeginPlay
  (Utilities|FlowControl|Sequence
    (:then_0
      ;[1 1 1] Set widget visibility
      (Rendering|SetVisibility (Variables|Default|GetWBP_Light) false false)
      ;[1 1 1] Get first person character Ref
      (bind _asbp_first_person_character (Utilities|Casting|CastToBP_FirstPersonCharacter (Game|GetPlayerCharacter 0)))
      (Variables|Default|SetBP_FirstPersonCharacter _asbp_first_person_character))))

(event EventInteract
  (bind _light_up (Variables|Default|GetLight_Up))
  (bind _light_down (Variables|Default|GetLight_Down))
  ;[1 1 1] Light on/off
  (Audio|PlaySound2D "/Game/BPARCHVIZ_COURSEFILES/THIRD_PART/AUDIOS/ClickSound.ClickSound" 1.0 1.0 0.0 0 0)
  (Utilities|FlowControl|FlipFlop
    (:A
      (bind _switch_off (Timeline|SwitchOff Play)
        (:Update
          (Transformation|SetRelativeRotation (Variables|Default|GetSwitch) (Math|Rotator|MakeRotator (* _switch_off -12.0) 0.0 0.0) false false)
          (Utilities|FlowControl|Delay 0.1)
          (Rendering|Components|Light|SetIntensity (Variables|Default|GetRectLight3) 0.0)
          (Rendering|Components|Light|SetIntensity _light_up 2.5e+03)
          (Rendering|Components|Light|SetIntensity _light_down 2.5e+03)
          (Rendering|Material|SetMaterial (Variables|Default|GetLight4) 1 "/Game/AiBIM_Content/Materials/Material_Instance/Glass/M_Glass_Inst.M_Glass_Inst"))))
    (:B
      (bind _switch_off_2 (Timeline|SwitchOn Play)
        (:Update
          (Transformation|SetRelativeRotation (Variables|Default|GetSwitch) (Math|Rotator|MakeRotator (* _switch_off_2 -12.0) 0.0 0.0) false false)
          (Utilities|FlowControl|Delay 0.1)
          (Rendering|Components|Light|SetIntensity (Variables|Default|GetRectLight) 1e+03)
          (Rendering|Components|Light|SetIntensity _light_up 1.5e+04)
          (Rendering|Components|Light|SetIntensity _light_down 5.5e+03)
          (Rendering|Material|SetMaterial (Variables|Default|GetLight1) 1 "/Game/AiBIM_Content/Materials/Material_Instance/LightEmitting/AiBIM_LED_Light.AiBIM_LED_Light"))))))

(fn ConstructionScript)