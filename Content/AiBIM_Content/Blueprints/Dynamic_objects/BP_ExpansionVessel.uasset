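; Expansion vessel actor that shows floating widgets when approached or interacted with.
; Overlapping CollisionBorder reveals the first widget, and leaving it hides both.
; WidgetInteraction reveals the second widget, which hides again through the first-person character's IsNotHitting dispatcher, bound on BeginPlay.
; BeginPlay also hides both widgets and creates and stores a WBP_CraneStrainerIcon instance, which is not displayed here.
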(event OnComponentBeginOverlap(Collisionborder)
  (params (OverlappedComponent :type Primitive%20Component%20Object%20Reference) (OtherActor :type Actor%20Object%20Reference) (OtherComp :type Primitive%20Component%20Object%20Reference) (OtherBodyIndex :type Integer) (bFromSweep :type Boolean) (SweepResult :type Hit%20Result%20Structure%20%28by%20ref%29))
  (Rendering|SetVisibility (Variables|Default|GetWidget) true false))

(event OnComponentEndOverlap(Collisionborder)
  (params (OverlappedComponent :type Primitive%20Component%20Object%20Reference) (OtherActor :type Actor%20Object%20Reference) (OtherComp :type Primitive%20Component%20Object%20Reference) (OtherBodyIndex :type Integer))
  (Rendering|SetVisibility (Variables|Default|GetWidget1) false false)
  (Rendering|SetVisibility (Variables|Default|GetWidget) false false))

(event Custom|Hide%20Widget
  (Rendering|SetVisibility (Variables|Default|GetWidget1) false false))

(event EventWidgetInteraction
  (Rendering|SetVisibility (Variables|Default|GetWidget1) true false))

(event EventBeginPlay
  ;[1 1 1] Floating Widgets
  (Utilities|FlowControl|Sequence
    (:then_0
      ;;[1 1 1] Create Tab widget
      (bind _returnvalue (UserInterface|CreateWidget "/Game/AiBIM_Content/Blueprints/Widgets/WBP_CraneStrainerIcon.WBP_CraneStrainerIcon_C"))
      (Variables|Default|SetWBP_ObjDisc _returnvalue))
    (:then_1
      ;;[1 1 1] Set widget visibility
      (Rendering|SetVisibility (Variables|Default|GetWidget) false false)
      (Rendering|SetVisibility (Variables|Default|GetWidget1) false false)
      (bind _asbp_first_person_character (Utilities|Casting|CastToBP_FirstPersonCharacter (Game|GetPlayerCharacter 0)))
      (Variables|Default|SetBP_FirstPersonCharacter _asbp_first_person_character))
    (:then_2
      (EventDispatchers|BindEventtoIsNotHitting (Variables|Default|GetBP_FirstPersonCharacter) (delegate Custom|Hide%20Widget)))))

(fn ConstructionScript)